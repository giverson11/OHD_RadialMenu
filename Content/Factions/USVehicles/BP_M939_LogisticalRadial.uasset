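; Blueprint for the US M939 logistics truck, a child vehicle that wires up interaction, radial menus and effects.
; The construction script registers three interact widgets on the hitbox mesh and maps separate radial menu tables to the driver and front-right seats.
; It also hands the exhaust emitter and engine audio to the vehicle FX component.
; Tick defers to the parent, then calls a cosmetic-event check without using its result.
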(event EventTick
  (params (DeltaSeconds :type Float%20%28single-precision%29))
  (|CallParentFunction DeltaSeconds)
  (Networking|CanExecuteCosmeticEvents))

(fn ConstructionScript
  (bind _vehicleinteractiblecomponent (Variables|Default|GetVehicleInteractibleComponent))
  (|CallParentFunction)
  (Default|SetInteractWidgets (Variables|Default|GetVehicleInteractibleComponent) (Utilities|Array|MakeArray (Variables|Default|GetWidget) (Variables|Default|GetWidget1) (Variables|Default|GetWidget2)) (Variables|Default|GetHitboxMesh))
  (Default|MapInternalRadialMenutoSeat _vehicleinteractiblecomponent (Variables|Default|GetDriverSeat) (Variables|Default|GetDriverRadialMenu))
  (Default|MapInternalRadialMenutoSeat _vehicleinteractiblecomponent (Variables|Default|GetS_FR_Seat) (Variables|Default|GetFrontRightRadialMenu))
  (Variables|/HDCore/Core/Vehicles/BP_HDVehicleFXComponent.BP_HDVehicleFXComponent_C|SetExhaustEmitterRefs (Variables|Default|GetVehicleFXComponent) (Utilities|Array|MakeArray (Variables|Default|GetExhaust%20VFX%20)))
  (Variables|/HDCore/Core/Vehicles/BP_HDVehicleFXComponent.BP_HDVehicleFXComponent_C|SetEngineAudioRef (Variables|Default|GetVehicleFXComponent) (Variables|Default|GetEngineAC)))

(fn InitiateInteractWidget
  (return (Utilities|Array|MakeArray (Variables|Default|GetWidget) (Variables|Default|GetWidget1) (Variables|Default|GetWidget2))))