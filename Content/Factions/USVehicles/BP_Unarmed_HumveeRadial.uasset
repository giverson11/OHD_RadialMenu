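; Unarmed US Humvee vehicle Blueprint with seat-specific radial menus, built on a parent vehicle class.
; Its construction script registers four interact widgets against the hitbox mesh and maps radial menu data tables to the driver, front-right and rear-right seats.
; It also hands the exhaust emitter and engine audio references to the vehicle FX component.
; Tick calls the parent and a cosmetic-events check, with no further logic.
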(event EventTick
  (params (DeltaSeconds :type Float%20%28single-precision%29))
  (|CallParentFunction DeltaSeconds)
  (Networking|CanExecuteCosmeticEvents))

(fn ConstructionScript
  (bind _vehicleinteractiblecomponent (Variables|Default|GetVehicleInteractibleComponent))
  (|CallParentFunction)
  (Default|SetInteractWidgets _vehicleinteractiblecomponent (Utilities|Array|MakeArray (Variables|Default|GetWidget) (Variables|Default|GetWidget1) (Variables|Default|GetWidget2) (Variables|Default|GetWidget3)) (Variables|Default|GetHitboxMesh))
  (Default|MapInternalRadialMenutoSeat _vehicleinteractiblecomponent (Variables|Default|GetDriverSeat) (Variables|Default|GetDriverRadialMenu))
  (Default|MapInternalRadialMenutoSeat _vehicleinteractiblecomponent (Variables|Default|GetS_FR_Seat) (Variables|Default|GetFrontRightRadialMenu))
  (Default|MapInternalRadialMenutoSeat _vehicleinteractiblecomponent (Variables|Default|GetS_RR_2_Seat) (Variables|Default|GetBackRight))
  (Variables|/HDCore/Core/Vehicles/BP_HDVehicleFXComponent.BP_HDVehicleFXComponent_C|SetExhaustEmitterRefs (Variables|Default|GetVehicleFXComponent) (Utilities|Array|MakeArray (Variables|Default|GetExhaust%20VFX%20)))
  (Variables|/HDCore/Core/Vehicles/BP_HDVehicleFXComponent.BP_HDVehicleFXComponent_C|SetEngineAudioRef (Variables|Default|GetVehicleFXComponent) (Variables|Default|GetEngineAC)))