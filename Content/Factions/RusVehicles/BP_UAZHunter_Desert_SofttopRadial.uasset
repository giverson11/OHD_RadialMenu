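; Desert soft-top radial UAZ Hunter vehicle Blueprint for the Russian faction, built on a parent vehicle class.
; Its construction script registers four interaction widgets with the interactible component and hands the exhaust emitter and engine audio to the vehicle FX component.
; Tick runs the parent tick, then calls the cosmetic-event check without using its result.
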(event EventTick
  (params (DeltaSeconds :type Float%20%28single-precision%29))
  (|CallParentFunction DeltaSeconds)
  (Networking|CanExecuteCosmeticEvents))

(fn ConstructionScript
  (|CallParentFunction)
  (Default|SetInteractWidgets (Variables|Default|GetInteractibleComponent) (Utilities|Array|MakeArray (Variables|Default|GetWidget) (Variables|Default|GetWidget1) (Variables|Default|GetWidget2) (Variables|Default|GetWidget3)))
  (Variables|/HDCore/Core/Vehicles/BP_HDVehicleFXComponent.BP_HDVehicleFXComponent_C|SetExhaustEmitterRefs (Variables|Default|GetVehicleFXComponent) (Utilities|Array|MakeArray (Variables|Default|GetExhaust%20VFX%20)))
  (Variables|/HDCore/Core/Vehicles/BP_HDVehicleFXComponent.BP_HDVehicleFXComponent_C|SetEngineAudioRef (Variables|Default|GetVehicleFXComponent) (Variables|Default|GetEngineAC)))