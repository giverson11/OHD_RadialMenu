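; Player character Blueprint, Radial variant, that toggles the player controller's interact widgets as the character becomes incapacitated or recovers.
; Tick, gated to cosmetic execution, polls IsIncapacitated and calls ToggleInteractWidgets on player controller 0: true when incapacitated, false once recovered and alive.
; Two DoOnce nodes re-arm each other so each change fires once.
; The polling is a marked placeholder until a Wounded/Revived dispatcher exists.
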(event EventBeginPlay
  (|CallParentFunction) ; This node is disabled and will not be called.\nDrag off pins to build functionality.
)

(event Collision|EventActorBeginOverlap
  (params (OtherActor :type Actor%20Object%20Reference)))

(event EventTick
  (params (DeltaSeconds :type Float%20%28single-precision%29))
  (bind _returnvalue (Game|GetPlayerController 0))
  (bind _asbp_hdplayer_controller_radial (Utilities|Casting|CastToBP_HDPlayerController_Radial _returnvalue))
  ;[1 0 0.04033] PLACEHOLDER Replace this when a Wounded/Revived dispatcher is implemented instead of checking on tick
  (|CallParentFunction DeltaSeconds)
  (Networking|CanExecuteCosmeticEvents
    (:True
      (if (Class|DFBaseCharacter|IsIncapacitated)
        (Utilities|FlowControl|DoOnce false :!label _label
          (:Completed
            (Default|CallToggleInteractWidgets _asbp_hdplayer_controller_radial true)
            (goto _label_2 Reset)))
        (else
          (Utilities|FlowControl|DoOnce true :!label _label_2
            (:Completed
              (if (Class|DFBaseCharacter|IsAlive)
                (Default|CallToggleInteractWidgets _asbp_hdplayer_controller_radial false)
                (goto _label Reset)))))))))

(fn ConstructionScript
  (|CallParentFunction))