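; Player controller component that shows, branches and hides the radial interaction menu, toggling mouse input and interact widgets with it.
; Menu choices run RadialTrigger objects, lazily constructed and cached per class, which also supply button states.
; The component relays server and owning-client RPCs to those triggers by class.
; Its tick, enabled on demand, either drives a Click Tick Release trigger or closes the menu when the player leaves interact range.
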(event Custom|FinishTrigger
  ;[1 0.5729 0.8987] On Tick Logic
  (Components|Tick|SetComponentTickEnabled false)
  (Default|FinishTrigger (Variables|RadialTrigger|GetActiveRadialTrigger) (Variables|Core|GetOwningController))
  (Variables|RadialTrigger|SetActiveRadialTrigger 0))

(event Custom|CancelTrigger
  ;[1 0.5729 0.8987] On Tick Logic
  (Components|Tick|SetComponentTickEnabled false)
  (Default|CancelTrigger (Variables|RadialTrigger|GetActiveRadialTrigger) (Variables|Core|GetOwningController))
  (Variables|RadialTrigger|SetActiveRadialTrigger 0))

(event Custom|CallServerRPCData
  (params (Owner :type Actor%20Object%20Reference) (RadialTriggerClass :type Radial%20Trigger%20Class%20Reference) (DataParameter :type Object%20Soft%20Object%20Reference) (ActionIndex :type Integer))
  ;[1 0.763 0.375] ClientToServerRPC's
  (CallFunction|ServerRPCData Owner RadialTriggerClass DataParameter ActionIndex))

(event Custom|ServerRPCIndex
  (params (RadialTriggerClass :type Radial%20Trigger%20Class%20Reference) (ActionIndex :type Integer))
  ;[1 0.763 0.375] ClientToServerRPC's
  (bind _value (RadialTrigger|GetRadialTriggerInstance RadialTriggerClass))
  (Default|ServerRPCIndex _value ActionIndex))

(event Custom|ServerStartTrigger
  (params (Owner :type Actor%20Object%20Reference) (RadialTriggerClass :type Radial%20Trigger%20Class%20Reference) (DataParameter :type Object%20Soft%20Object%20Reference) (ClassParameter :type Object%20Soft%20Class%20Reference) (ActionIndex :type Integer))
  ;[1 0.763 0.375] ClientToServerRPC's
  (bind _value (RadialTrigger|GetRadialTriggerInstance RadialTriggerClass))
  (Default|ServerRPCBase _value Owner DataParameter ClassParameter ActionIndex))

(event Custom|CallServerRPCBase
  (params (Owner :type Actor%20Object%20Reference) (RadialTriggerClass :type Radial%20Trigger%20Class%20Reference) (DataParameter :type Object%20Soft%20Object%20Reference) (ClassParameter :type Object%20Soft%20Class%20Reference) (ActionIndex :type Integer))
  ;[1 0.763 0.375] ClientToServerRPC's
  (CallFunction|ServerStartTrigger Owner RadialTriggerClass DataParameter ClassParameter ActionIndex))

(event Custom|CallServerRPCIndex
  (params (RadialTriggerClass :type Radial%20Trigger%20Class%20Reference) (ActionIndex :type Integer))
  ;[1 0.763 0.375] ClientToServerRPC's
  (CallFunction|ServerRPCIndex RadialTriggerClass ActionIndex))

(event Custom|ServerRPCClass
  (params (Owner :type Actor%20Object%20Reference) (RadialTriggerClass :type Radial%20Trigger%20Class%20Reference) (ClassParameter :type Object%20Soft%20Class%20Reference) (ActionIndex :type Integer))
  ;[1 0.763 0.375] ClientToServerRPC's
  (bind _value (RadialTrigger|GetRadialTriggerInstance RadialTriggerClass))
  (Default|ServerRPCClass _value Owner ClassParameter ActionIndex))

(event Custom|CallServerRPCClass
  (params (Owner :type Actor%20Object%20Reference) (RadialTriggerClass :type Radial%20Trigger%20Class%20Reference) (ClassParameter :type Object%20Soft%20Class%20Reference) (ActionIndex :type Integer))
  ;[1 0.763 0.375] ClientToServerRPC's
  (CallFunction|ServerRPCClass Owner RadialTriggerClass ClassParameter ActionIndex))

(event Custom|ClientRPCBase
  (params (RadialTrigger :type Radial%20Trigger%20Class%20Reference) (ActionIndex :type Integer))
  ;[0.5938 0.7129 1] Server to Owning Client RPC's
  (bind _value (RadialTrigger|GetRadialTriggerInstance RadialTrigger))
  (Default|OwningClientRPCBase _value ActionIndex))

(event Custom|CallClientRPCMessage
  (params (RadialTriggerClass :type Radial%20Trigger%20Class%20Reference) (Message :type String))
  ;[0.5938 0.7129 1] Server to Owning Client RPC's
  (CallFunction|CallClientRPCMessage RadialTriggerClass Message))

(event Custom|ClientRPCMessage
  (params (RadialTriggerClass :type Radial%20Trigger%20Class%20Reference) (Message :type String))
  ;[0.5938 0.7129 1] Server to Owning Client RPC's
  (bind _value (RadialTrigger|GetRadialTriggerInstance RadialTriggerClass))
  (Default|OwningClientRPCMessage _value Message))

(event Custom|CallClientRPCBase
  (params (RadialTriggerClass :type Radial%20Trigger%20Class%20Reference) (ActionIndex :type Integer))
  ;[0.5938 0.7129 1] Server to Owning Client RPC's
  (CallFunction|ClientRPCBase RadialTriggerClass ActionIndex))

(event Custom|ServerRPCOwner
  (params (RadialTriggerClass :type Radial%20Trigger%20Class%20Reference) (Owner :type Actor%20Object%20Reference))
  ;[1 0.763 0.375] ClientToServerRPC's
  (bind _value (RadialTrigger|GetRadialTriggerInstance RadialTriggerClass))
  (Default|ServerRPCOwner _value Owner))

(event Custom|CallServerRPCOwner
  (params (RadialTriggerClass :type Radial%20Trigger%20Class%20Reference) (Owner :type Actor%20Object%20Reference))
  ;[1 0.763 0.375] ClientToServerRPC's
  (CallFunction|ServerRPCOwner RadialTriggerClass Owner))

(event Custom|ServerRPCData
  (params (Owner :type Actor%20Object%20Reference) (RadialTriggerClass :type Radial%20Trigger%20Class%20Reference) (DataParameter :type Object%20Soft%20Object%20Reference) (ActionIndex :type Integer))
  ;[1 0.763 0.375] ClientToServerRPC's
  (bind _value (RadialTrigger|GetRadialTriggerInstance RadialTriggerClass))
  (Default|ServerRPCData _value Owner DataParameter ActionIndex))

(event EventBeginPlay
  (bind _asbp_hdplayer_controller_radial (Utilities|Casting|CastToBP_HDPlayerController_Radial (Components|GetOwner)))
  (Variables|Core|SetOwningController _asbp_hdplayer_controller_radial))

(event EventTick
  (params (DeltaSeconds :type Float%20%28single-precision%29))
  (bind _owningcontroller (Variables|Core|GetOwningController))
  ;[1 0.5729 0.8987] On Tick Logic
  (if (CallFunction|IsRadialTriggerTicking)
    (Default|OnTick (Variables|RadialTrigger|GetActiveRadialTrigger) (Variables|Core|GetOwningController) DeltaSeconds)
    (else
      (bind _returnvalue (Class|PrimitiveComponent|SphereOverlapComponent (Variables|Default|GetTargetMeshComponent) (Transformation|GetActorLocation (Pawn|GetControlledPawn _owningcontroller)) (Variables|/RadialMenu/Core/BP_HDPlayerController_Radial.BP_HDPlayerController_Radial_C|GetInteractDistance _owningcontroller) true false false)) ; Disables Radial Menu if Player gets far enough away from a interactive object
      (if (not _returnvalue)
        (RadialMenu|HideRadialMenu)))))

(fn DisplayRadialMenu
  (params (Owner :type Actor%20Object%20Reference) (Radial%20Data :type S%20Radial%20Menu%20Info%20Structure) (DistanceCheckEnabled :type Boolean) (TargetMeshComponent :type Mesh%20Component%20Object%20Reference))
  (bind _radialmenu (Variables|Widget|GetRadialMenu))
  (if (CallFunction|IsRadialTriggerTicking)
    (CallFunction|CancelTrigger))
  (if (not (Variables|Core|GetInteracting))
    (if DistanceCheckEnabled
      (Variables|Default|SetTargetMeshComponent TargetMeshComponent)
      (Class|ActorComponent|SetComponentTickInterval (Variables|Core|GetDistanceCheckTickRate))
      (Components|Tick|SetComponentTickEnabled true))
    (Default|CallToggleInteractWidgets (Variables|Core|GetOwningController) true) ; Hide interact widgets when Radial menu is displayed
    (Input|SetupControllerInput)
    (Default|CallOnRadialMenuStateChanged true)
    (Utilities|IsValid _radialmenu
      (:Is%20Valid
        (Default|DisplayNewRadialMenu _radialmenu Radial%20Data Owner)
        (Widget|SetVisibility _radialmenu "SelfHitTestInvisible"))
      (:Is%20Not%20Valid
        (RadialMenu|LoadRadialMenu Owner Radial%20Data)))
    (Variables|Core|SetRadialMenuOwner Owner)
    (return)))

(fn LoadRadialMenu
  (params (Owner :type Actor%20Object%20Reference) (Radial%20Data :type S%20Radial%20Menu%20Info%20Structure))
  (bind _returnvalue (UserInterface|CreateWidget "/RadialMenu/Core/Widgets/RadialMenu/Radial_Base_RDC.Radial_Base_RDC_C" (Variables|Core|GetOwningController) Owner Radial%20Data))
  (UserInterface|Viewport|AddtoPlayerScreen _returnvalue)
  (Variables|Widget|SetRadialMenu _returnvalue))

(fn HideRadialMenu
  (bind _radialmenu (Variables|Widget|GetRadialMenu))
  (if (CallFunction|IsRadialTriggerTicking)
    (CallFunction|CancelTrigger))
  (if (Variables|Core|GetInteracting)
    (if (Class|ActorComponent|IsComponentTickEnabled)
      (Components|Tick|SetComponentTickEnabled false))
    (Utilities|IsValid _radialmenu
      (:Is%20Valid
        (Default|RemoveRadialMenu _radialmenu)
        (Widget|SetVisibility _radialmenu "Collapsed")
        (Input|ResetControllerInput)
        (Default|CallToggleInteractWidgets (Variables|Core|GetOwningController) false)
        (Default|CallOnRadialMenuStateChanged false))
      (:Is%20Not%20Valid
        _))
    (Variables|Core|SetRadialMenuOwner 0)
    (return)))

(fn CallRadialTrigger
  (params (Owner :type Actor%20Object%20Reference) (RadialTrigger :type Radial%20Trigger%20Class%20Reference) (RadialTriggerDataParameter :type Object%20Soft%20Object%20Reference) (RadialTriggerClassParameter :type Object%20Soft%20Class%20Reference) (ActionIndex :type Integer))
  (bind _value (RadialTrigger|GetRadialTriggerInstance RadialTrigger))
  (Default|StartRadialTrigger _value Owner RadialTriggerDataParameter RadialTriggerClassParameter ActionIndex)
  ;[1 0.01504 0] On Tick logic is experimental and untested, might be a good idea to only support single activation
  (switch Utilities|FlowControl|Switch|SwitchonE_RadialTriggerType (Variables|/RadialMenu/Core/RadialTriggers/RadialTrigger.RadialTrigger_C|GetTriggerType _value)
    (:NewEnumerator0
      (RadialMenu|HideRadialMenu))
    (:NewEnumerator1
      (RadialMenu|HideRadialMenu)
      (bind _output_get (Variables|RadialTrigger|SetActiveRadialTrigger _value))
      (Class|ActorComponent|SetComponentTickInterval (Variables|/RadialMenu/Core/RadialTriggers/RadialTrigger.RadialTrigger_C|GetTickRate _output_get))
      (Components|Tick|SetComponentTickEnabled true))))

(fn LoadRadialTrigger
  (params (RadialTriggerClass :type Radial%20Trigger%20Class%20Reference%20%28by%20ref%29))
  (bind _returnvalue (Components|GetOwner))
  (bind _asbp_hdplayer_controller_radial (Utilities|Casting|CastToBP_HDPlayerController_Radial _returnvalue))
  (bind _returnvalue_2 (Game|ConstructObjectfromClass RadialTriggerClass _returnvalue _asbp_hdplayer_controller_radial self))
  (Utilities|Map|Add (Variables|RadialTrigger|GetRadialTriggerMap) RadialTriggerClass _returnvalue_2)
  (return _returnvalue_2))

(fn SetupControllerInput
  (bind _owningcontroller (Variables|Core|GetOwningController))
  (Variables|Core|SetInteracting true)
  (CallFunction|CenterMousePosition 0 _owningcontroller)
  (Input|SetInputModeGameandUI _owningcontroller (Variables|Widget|GetRadialMenu) "DoNotLock" false)
  (Variables|/Script/Engine.PlayerController|SetbShowMouseCursor _owningcontroller true))

(fn ResetControllerInput
  (bind _owningcontroller (Variables|Core|GetOwningController))
  (Variables|Core|SetInteracting false)
  (Input|SetInputModeGameOnly _owningcontroller)
  (Variables|/Script/Engine.PlayerController|SetbShowMouseCursor _owningcontroller false))

(fn GetRadialTriggerInstance
  (params (RadialTriggerClass :type Radial%20Trigger%20Class%20Reference%20%28by%20ref%29))
  (bind _radialtriggermap (Variables|RadialTrigger|GetRadialTriggerMap))
  (bind (_value _returnvalue) (Utilities|Map|Find _radialtriggermap RadialTriggerClass))
  (if _returnvalue
    (return _value)
    (else
      (bind _output_get (RadialTrigger|LoadRadialTrigger RadialTriggerClass))
      (return _output_get))))

(fn GetRadialMenuOwner
  (return (Variables|Core|GetRadialMenuOwner)))

(fn GetRadialTriggerActivationState
  (params (Owner :type Actor%20Object%20Reference) (RadialTrigger :type Radial%20Trigger%20Class%20Reference) (RadialTriggerDataParameter :type Object%20Soft%20Object%20Reference) (RadialTriggerClassParameter :type Object%20Soft%20Class%20Reference) (ActionIndex :type Integer))
  (bind _value (RadialTrigger|GetRadialTriggerInstance RadialTrigger))
  (bind (_radialbuttonstate _disabledmessage) (Default|SetRadialButtonState _value Owner RadialTriggerDataParameter RadialTriggerClassParameter ActionIndex))
  (return _radialbuttonstate _disabledmessage))

(fn BranchtoNewRadialMenu
  (params (NewRadialMenu :type Data%20Table%20Row%20Handle%20Structure))
  (bind _radialmenu (Variables|Widget|GetRadialMenu))
  (Utilities|IsValid _radialmenu
    (:Is%20Valid
      (bind _returnvalue (Utilities|GetDataTableRow (.datatable NewRadialMenu) (.rowname NewRadialMenu))
        (:then
          (Default|BranchtoNewRadialMenu _radialmenu _returnvalue))))))

(fn IsRadialTriggerTicking
  (return (Utilities|IsValid (Variables|RadialTrigger|GetActiveRadialTrigger))))