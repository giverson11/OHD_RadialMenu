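; Vehicle interactible component that gives each seat its own internal radial menu.
; An event registers a data table row handle per seat in a map, only where cosmetic events can execute and the table is valid.
; The display function looks up the seat's row and shows it through the radial menu component with the owning actor, returning whether it succeeded.
; Helper functions query or fetch a seat's mapping.
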(event Custom|MapInternalRadialMenuToSeat
  (params (Seat :type BP%20HD%20Vehicle%20Seat%20Attachment%20Player%20Object%20Reference%20%28by%20ref%29) (DataTable :type Data%20Table%20Row%20Handle%20Structure%20%28by%20ref%29))
  (Networking|CanExecuteCosmeticEvents
    (:True
      (Utilities|IsValid (.DataTable (Utilities|Struct|BreakDataTableRowHandle DataTable))
        (:Is%20Valid
          (Utilities|Map|Add (Variables|Default|GetRadialMapBySeat) Seat DataTable))))))

(event EventBeginPlay
  (|CallParentFunction) ; This node is disabled and will not be called.\nDrag off pins to build functionality.
)

(event EventTick
  (params (DeltaSeconds :type Float%20%28single-precision%29))
  (|CallParentFunction DeltaSeconds) ; This node is disabled and will not be called.\nDrag off pins to build functionality.
)

(fn DisplayInternalRadialMenubySeat
  (params (Seat :type BP%20HD%20Vehicle%20Seat%20Attachment%20Player%20Object%20Reference%20%28by%20ref%29))
  (bind (_radialmenucomp _isvalid) (CallFunction|GetRadialMenuComp))
  (bind _radialmapbyseat (Variables|Default|GetRadialMapBySeat))
  (bind (_value _returnvalue) (Utilities|Map|Find _radialmapbyseat Seat))
  (if _returnvalue
    (LocalVariables|SetRadialMenuData _value)
    (if _isvalid
      (bind _returnvalue_2 (Utilities|GetDataTableRow (.datatable (LocalVariables|GetRadialMenuData)) (.rowname (LocalVariables|GetRadialMenuData)))
        (:then
          (Default|DisplayRadialMenu _radialmenucomp (Components|GetOwner) _returnvalue_2 false)
          (return true))
        (:RowNotFound
          _))))
  (return false))

(fn IsSeatMappedtoRadialMenu
  (params (Seat :type BP%20HD%20Vehicle%20Seat%20Attachment%20Player%20Object%20Reference%20%28by%20ref%29))
  (return (.ReturnValue (Utilities|Map|Find (Variables|Default|GetRadialMapBySeat) Seat))))

(fn GetRadialMenubySeat
  (params (Seat :type BP%20HD%20Vehicle%20Seat%20Attachment%20Player%20Object%20Reference%20%28by%20ref%29))
  (bind _radialmapbyseat (Variables|Default|GetRadialMapBySeat))
  (bind (_value _returnvalue) (Utilities|Map|Find _radialmapbyseat Seat))
  (return _value _returnvalue))