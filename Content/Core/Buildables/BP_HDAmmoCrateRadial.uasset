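; Buildable ammo crate that opens a radial menu when a player on the owning team interacts with it.
; Interaction goes through the InteractibleComponent, which must not be sleeping, and the construction script assigns its interact widget.
; On health or build changes, where cosmetic events can run, it initializes or enables that widget above a build-percentage health threshold and disables it otherwise.
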(event EventBeginPlay
  (|CallParentFunction))

(event Collision|EventActorBeginOverlap
  (params (OtherActor :type Actor%20Object%20Reference)))

(event EventTick
  (params (DeltaSeconds :type Float%20%28single-precision%29))
  (|CallParentFunction DeltaSeconds))

(event EventInteract
  (params (InstigatingController :type BP%20HD%20Player%20Controller%20Base%20Object%20Reference))
  (if (and (== (Variables|Default|GetOwningTeam) (Class|DFBlueprintFunctions|GetTeamNum InstigatingController)) (not (Default|IsSleeping (Variables|Default|GetInteractibleComponent))))
    (Default|DisplayRadialMenu (Variables|Default|GetInteractibleComponent))))

(event EventHandleHealthChangeBuildLevel
  (params (Old%20Health :type Float%20%28single-precision%29) (New%20Health :type Float%20%28single-precision%29) (Build%20Status :type Integer))
  (bind _interactiblecomponent (Variables|Default|GetInteractibleComponent))
  (|CallParentFunction Old%20Health New%20Health Build%20Status)
  (Networking|CanExecuteCosmeticEvents
    (:True
      (if (> New%20Health (* (Utilities|Array|Get(acopy) (Variables|Default|GetBuildPercentages) 5) (Variables|Default|GetMaximumHealth)))
        (if (Default|IsInitialized _interactiblecomponent)
          (Default|EnableInteractWidget _interactiblecomponent)
          (else
            (Default|Initialize _interactiblecomponent)))
        (else
          (Default|DisableInteractWidget _interactiblecomponent))))))

(fn ConstructionScript
  (|CallParentFunction)
  (Default|SetInteractWidgets (Variables|Default|GetInteractibleComponent) (Utilities|Array|MakeArray (Variables|Default|GetWidget))))