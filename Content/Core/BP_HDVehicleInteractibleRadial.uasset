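; Vehicle Blueprint that offers a radial interaction menu to players on the same team.
; Interact compares team numbers, then has VehicleInteractibleComponent display the menu.
; A cosmetic-only seat-change binding ends the local player's interaction and toggles interact widgets through BP_HDPlayerController_Radial on vehicle entry and exit.
; Vehicle destruction puts a sleep lock on the component, though the live Interact path does not check sleep state.
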(event Custom|OnChangeSeat
  (params (Player :type Player%20State%20Object%20Reference) (ToSeat :type Arc%20Vehicle%20Seat%20Config%20Object%20Reference) (FromSeat :type Arc%20Vehicle%20Seat%20Config%20Object%20Reference) (SeatChangeEvent :type EArcVehicleSeatChangeType%20Enum :default "Invalid"))
  (bind _ownerpc (CallFunction|GetPlayerControllerfromPlayerState Player))
  ;[1 1 1] If Player Enters or exits vehicle, hide interact widgets
  (Utilities|IsValid _ownerpc
    (:Is%20Valid
      (if (Pawn|IsLocalPlayerController _ownerpc)
        (bind _asbp_hdplayer_controller_radial (Utilities|Casting|CastToBP_HDPlayerController_Radial _ownerpc))
        (Default|EndInteraction _asbp_hdplayer_controller_radial)
        (switch Utilities|FlowControl|Switch|SwitchonEArcVehicleSeatChangeType SeatChangeEvent
          (:EnterVehicle
            (Default|CallToggleInteractWidgets _asbp_hdplayer_controller_radial true))
          (:ExitVehicle
            (Default|CallToggleInteractWidgets _asbp_hdplayer_controller_radial false)))))))

(event EventVehicleDestroyedBP
  (params (KillingDamage :type Float%20%28single-precision%29) (DamageEvent :type Damage%20Event%20Structure%20%28by%20ref%29) (InstigatingPawn :type Pawn%20Object%20Reference) (DamageCauser :type Actor%20Object%20Reference))
  (|CallParentFunction KillingDamage DamageEvent InstigatingPawn DamageCauser)
  (Default|AcquireSleepLock (Variables|Default|GetVehicleInteractibleComponent)))

(event Collision|EventActorBeginOverlap
  (params (OtherActor :type Actor%20Object%20Reference)))

(event EventTick
  (params (DeltaSeconds :type Float%20%28single-precision%29))
  (|CallParentFunction DeltaSeconds))

(event EventBeginPlay
  (|CallParentFunction)
  (Networking|CanExecuteCosmeticEvents
    (:True
      (EventDispatchers|BindEventtoOnNotifyPlayerSeatChangeEventDelegate (delegate Custom|OnChangeSeat)))))

(event EventUsed
  (params (Invoker :type Actor%20Object%20Reference)))

(event EventInteract
  (params (InstigatingController :type BP%20HD%20Player%20Controller%20Base%20Object%20Reference))
  (if (== (Class|DFBlueprintFunctions|GetTeamNum self) (Class|DFBlueprintFunctions|GetTeamNum InstigatingController))
    (Default|DisplayRadialMenu (Variables|Default|GetVehicleInteractibleComponent))))

(fn ConstructionScript
  (|CallParentFunction))