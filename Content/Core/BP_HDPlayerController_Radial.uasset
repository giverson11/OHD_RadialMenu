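; Player controller that layers a radial interaction menu onto character and vehicle input.
; MountWeapon opens the menu from the current loadout's data table row, while death, pause or deploy menu toggling hides it.
; Fire and Aim finish or cancel ticking radial triggers, otherwise driving weapon, shovel and medical item actions.
; Use sends interact messages to the current vehicle or a camera-traced actor, with a vehicle-entry trace fallback for other pawns.
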(event Custom|End%20Interaction
  (Default|HideRadialMenu (Variables|Default|GetRadialMenu)))

(event EventCharacterDeath
  (params (VictimPawn :type Pawn%20Object%20Reference) (VictimController :type Controller%20Object%20Reference) (KillingDamage :type Float%20%28single-precision%29) (DamageEvent :type Damage%20Event%20Structure%20%28by%20ref%29) (InstigatingPawn :type Pawn%20Object%20Reference) (DamageCauser :type Actor%20Object%20Reference))
  ;[1 1 1] Removes Radial Menu and Hides Interact Widgets on Death
  (|CallParentFunction VictimPawn VictimController KillingDamage DamageEvent InstigatingPawn DamageCauser)
  (bind _asbp_hdplayer_character_base (Utilities|Casting|CastToBP_HDPlayerCharacterBase VictimPawn)) ; If player is incapacitated when killed, widgets are already hidden so no need to hide
  (if (Class|DFBaseCharacter|IsIncapacitated _asbp_hdplayer_character_base)
    _
    (else
      (Default|CallToggleInteractWidgets true)))
  (CallFunction|EndInteraction))

(event Input|ActionEvents|InputActionFire
  (params (Key :type Key%20Structure :default "None"))
  (bind _radialmenu (Variables|Default|GetRadialMenu))
  (:Pressed
    ;[1 1 1] Interaction Fire Changes
    ;;[1 0 0] FiringBug
    (if (Default|IsRadialTriggerTicking _radialmenu)
      (Default|FinishTrigger _radialmenu) ; Will Still Fire Weapon when left clicking. \nFire input is probably being triggered is weapon alongside from the controller somewhere in c++\nNeed to fix this if you want tick based radial triggers
      (else
        (bind _asbp_hdplayer_character_base (Utilities|Casting|CastToBP_HDPlayerCharacterBase (Pawn|GetControlledPawn)))
        (Utilities|FlowControl|Sequence
          (:then_0
            (bind _asbp_hdweap_shovel_base (Utilities|Casting|CastToBP_HDWeap_ShovelBase (Class|DFBaseCharacter|GetEquippedItem _asbp_hdplayer_character_base))
              (:then
                (Default|Construct _asbp_hdweap_shovel_base))
              (:CastFailed
                (bind _asbp_hdweap_medical_base (Utilities|Casting|CastToBP_HDWeap_MedicalBase (Class|DFBaseCharacter|GetEquippedItem _asbp_hdplayer_character_base)))
                (Default|PrimaryFire _asbp_hdweap_medical_base))))
          (:then_1
            (Default|OnPCFirePressed _asbp_hdplayer_character_base))))))
  (:Released
    (if (not (Variables|/RadialMenu/Core/Components/BP_HDRadialMenuComponent.BP_HDRadialMenuComponent_C|GetInteracting (Variables|Default|GetRadialMenu)))
      (bind _asbp_hdplayer_character_base_2 (Utilities|Casting|CastToBP_HDPlayerCharacterBase (Pawn|GetControlledPawn)))
      (Default|OnPCFireReleased _asbp_hdplayer_character_base_2))))

(event Input|ActionEvents|InputActionMountWeapon
  (params (Key :type Key%20Structure :default "None"))
  ;[1 1 1] Base Radial System (Needs new keybind)
  (:Pressed
    (bind _asbp_hdplayer_character (Utilities|Casting|CastToBP_HDPlayerCharacter (Pawn|GetControlledPawn))
      (:then
        (Utilities|IsValid (Variables|/Script/HDMain.HDPlayerCharacter|GetCurrentLoadout _asbp_hdplayer_character)
          (:Is%20Valid
            (Utilities|IsValid (.datatable (Variables|/Script/HDMain.HDKit|GetRadialMenuData (Variables|/Script/HDMain.HDPlayerCharacter|GetCurrentLoadout _asbp_hdplayer_character)))
              (:Is%20Valid
                (bind _returnvalue (Utilities|GetDataTableRow (.datatable (Variables|/Script/HDMain.HDKit|GetRadialMenuData (Variables|/Script/HDMain.HDPlayerCharacter|GetCurrentLoadout _asbp_hdplayer_character))) (.rowname (Variables|/Script/HDMain.HDKit|GetRadialMenuData (Variables|/Script/HDMain.HDPlayerCharacter|GetCurrentLoadout _asbp_hdplayer_character))))
                  (:then
                    (Default|DisplayRadialMenu (Variables|Default|GetRadialMenu) (Pawn|GetControlledPawn) _returnvalue false))))))))
      (:CastFailed
        (bind _asbp_hdwheeled_vehicle_base (Utilities|Casting|CastToBP_HDWheeledVehicleBase (Pawn|GetControlledPawn)))
        (bind _ashdplayer_state (Utilities|Casting|CastToHDPlayerState (Variables|/Script/ArcVehicles.ArcVehicleSeatConfig|GetPlayerInSeat (Variables|/HDCore/Core/Vehicles/BP_HDWheeledVehicleBase.BP_HDWheeledVehicleBase_C|GetDriverSeat _asbp_hdwheeled_vehicle_base))))
        (bind _returnvalue_2 (Utilities|GetDataTableRow (.datatable (Variables|/Script/HDMain.HDKit|GetRadialMenuData (Variables|/Script/HDMain.HDPlayerState|GetCurrentLoadout _ashdplayer_state))) (.rowname (Variables|/Script/HDMain.HDKit|GetRadialMenuData (Variables|/Script/HDMain.HDPlayerState|GetCurrentLoadout _ashdplayer_state))))
          (:then
            (Default|DisplayRadialMenu (Variables|Default|GetRadialMenu) (Pawn|GetControlledPawn) _returnvalue_2 false))))))
  (:Released
    (if (not (Default|IsRadialTriggerTicking (Variables|Default|GetRadialMenu))) ; Makes sure tick based radial triggers dont cancel on release
      (CallFunction|EndInteraction))))

(event Input|ActionEvents|InputActionAimToggle
  (params (Key :type Key%20Structure :default "None"))
  (bind _radialmenu (Variables|Default|GetRadialMenu))
  (:Pressed
    ;[1 1 1] Interaction Aim changes
    (if (Variables|/RadialMenu/Core/Components/BP_HDRadialMenuComponent.BP_HDRadialMenuComponent_C|GetInteracting (Variables|Default|GetRadialMenu))
      (CallFunction|EndInteraction)
      (elif (Default|IsRadialTriggerTicking _radialmenu)
        (Default|CancelTrigger _radialmenu)
        (else
          (bind _asbp_hdplayer_character_base (Utilities|Casting|CastToBP_HDPlayerCharacterBase (Pawn|GetControlledPawn)))
          (if (Utilities|DoesObjectImplementInterface (Class|DFBaseCharacter|GetEquippedItem _asbp_hdplayer_character_base) "/RadialMenu/Core/Components/IF_Interactible.IF_Interactible_C")
            (Class|IFInteractible|Interact(Message) (Class|DFBaseCharacter|GetEquippedItem _asbp_hdplayer_character_base) self)
            (else
              (bind _asbp_hdweap_shovel_base (Utilities|Casting|CastToBP_HDWeap_ShovelBase (Class|DFBaseCharacter|GetEquippedItem _asbp_hdplayer_character_base))
                (:then
                  (Default|Deconstruct _asbp_hdweap_shovel_base)
                  (Default|OnPCFirePressed _asbp_hdplayer_character_base))
                (:CastFailed
                  (bind _asbp_hdweap_medical_base (Utilities|Casting|CastToBP_HDWeap_MedicalBase (Class|DFBaseCharacter|GetEquippedItem _asbp_hdplayer_character_base))
                    (:then
                      (if (Variables|/HDCore/Core/Items/BP_HDWeap_MedicalBase.BP_HDWeap_MedicalBase_C|GetAltFIreEnabled _asbp_hdweap_medical_base)
                        (Default|AltFire _asbp_hdweap_medical_base)
                        (Default|OnPCFirePressed _asbp_hdplayer_character_base)))
                    (:CastFailed
                      ;[1 0 0] Probably Don't need this for base controller
                      (Class|DFBaseCharacter|AimToggle _asbp_hdplayer_character_base)))))))))))
  (:Released
    (bind _asbp_hdplayer_character_base_2 (Utilities|Casting|CastToBP_HDPlayerCharacterBase (Pawn|GetControlledPawn)))
    (bind _asbp_hdweap_medical_base_2 (Utilities|Casting|CastToBP_HDWeap_MedicalBase (Class|DFBaseCharacter|GetEquippedItem _asbp_hdplayer_character_base_2)))
    (if (Variables|/HDCore/Core/Items/BP_HDWeap_MedicalBase.BP_HDWeap_MedicalBase_C|GetAltFIreEnabled _asbp_hdweap_medical_base_2)
      (Default|OnPCFireReleased _asbp_hdplayer_character_base))))

(event Input|ActionEvents|InputActionUse
  (params (Key :type Key%20Structure :default "None"))
  (bind _returnvalue (Pawn|GetControlledPawn))
  (bind _returnvalue_2 (Transformation|GetActorLocation _returnvalue))
  (bind _returnvalue_3 (Actor|GetComponentbyClass _returnvalue "/Script/ArcVehicles.ArcVehiclePlayerSeatComponent"))
  (bind _currentseatconfig (Variables|/Script/ArcVehicles.ArcVehiclePlayerSeatComponent|GetCurrentSeatConfig _returnvalue_3))
  (:Pressed
    (if (not (Variables|/RadialMenu/Core/Components/BP_HDRadialMenuComponent.BP_HDRadialMenuComponent_C|GetInteracting (Variables|Default|GetRadialMenu)))
      (bind _asarc_base_vehicle (Utilities|Casting|CastToArcBaseVehicle _returnvalue)
        (:then
          ;[1 1 1] Interact (This probably should replace Use eventually)
          (Class|IFInteractible|Interact(Message) _asarc_base_vehicle self))
        (:CastFailed
          (Utilities|IsValid _returnvalue_3
            (:Is%20Valid
              (if (Class|ArcVehicleBPFunctionLibrary|IsSeatRefValid _currentseatconfig)
                (Class|IFInteractible|Interact(Message) (Class|ArcVehicleBPFunctionLibrary|GetVehiclefromSeatConfig _currentseatconfig) self)
                (else
                  (bind _asdfbase_player_character (Utilities|Casting|CastToDFBasePlayerCharacter _returnvalue :!label _label)
                    (:then
                      (Class|DFBasePlayerCharacter|Use _asdfbase_player_character)
                      (bind (_outhit _returnvalue_4) (Collision|LineTraceByChannel (Transformation|GetWorldLocation (Class|DFBasePlayerCharacter|GetCamera1P _asdfbase_player_character)) (+ (Transformation|GetWorldLocation (Class|DFBasePlayerCharacter|GetCamera1P _asdfbase_player_character)) (* (Math|Vector|GetForwardVector (Class|DFBasePlayerCharacter|GetCamera1P _asdfbase_player_character)) (Variables|Interaction|GetInteractDistance))) "TraceTypeQuery1" false (Utilities|Array|MakeArray (Pawn|GetControlledPawn)) "ForDuration"))
                      (if _returnvalue_4
                        (Class|IFInteractible|Interact(Message) (.HitActor (Collision|BreakHitResult _outhit)) self)))
                    (:CastFailed
                      (bind (_outhit_2 _returnvalue_5) (Collision|LineTraceForObjects _returnvalue_2 (+ _returnvalue_2 (* (Math|Vector|GetForwardVector (Actor|GetComponentbyClass _returnvalue "/Script/Engine.CameraComponent")) 5e+02)) (Utilities|Array|MakeArray "ObjectTypeQuery5") false 0 "ForDuration"))
                      (if _returnvalue_5
                        (bind _asarc_base_vehicle_2 (Utilities|Casting|CastToArcBaseVehicle (.HitActor (Collision|BreakHitResult _outhit_2))))
                        (Networking|SwitchHasAuthority
                          (:Authority
                            (Class|ArcBaseVehicle|RequestEnterAnySeat _asarc_base_vehicle_2 (Variables|Default|GetPlayerState)))
                          (:Remote
                            (CallFunction|ServerTryGetinVehicle _asarc_base_vehicle_2)))))))))
            (:Is%20Not%20Valid
              (goto _label))))))))

(event Input|ActionEvents|InputActionAim
  (params (Key :type Key%20Structure :default "None"))
  (bind _radialmenu (Variables|Default|GetRadialMenu))
  (:Pressed
    ;[1 1 1] Interaction Aim changes
    (if (Variables|/RadialMenu/Core/Components/BP_HDRadialMenuComponent.BP_HDRadialMenuComponent_C|GetInteracting (Variables|Default|GetRadialMenu))
      (CallFunction|EndInteraction)
      (elif (Default|IsRadialTriggerTicking _radialmenu)
        (Default|CancelTrigger _radialmenu)
        (else
          (bind _asbp_hdplayer_character_base (Utilities|Casting|CastToBP_HDPlayerCharacterBase (Pawn|GetControlledPawn)))
          (if (Utilities|DoesObjectImplementInterface (Class|DFBaseCharacter|GetEquippedItem _asbp_hdplayer_character_base) "/RadialMenu/Core/Components/IF_Interactible.IF_Interactible_C")
            (Class|IFInteractible|Interact(Message) (Class|DFBaseCharacter|GetEquippedItem _asbp_hdplayer_character_base) self)
            (else
              (bind _asbp_hdweap_shovel_base (Utilities|Casting|CastToBP_HDWeap_ShovelBase (Class|DFBaseCharacter|GetEquippedItem _asbp_hdplayer_character_base))
                (:then
                  (Default|Deconstruct _asbp_hdweap_shovel_base)
                  (Default|OnPCFirePressed _asbp_hdplayer_character_base))
                (:CastFailed
                  (bind _asbp_hdweap_medical_base (Utilities|Casting|CastToBP_HDWeap_MedicalBase (Class|DFBaseCharacter|GetEquippedItem _asbp_hdplayer_character_base))
                    (:then
                      (if (Variables|/HDCore/Core/Items/BP_HDWeap_MedicalBase.BP_HDWeap_MedicalBase_C|GetAltFIreEnabled _asbp_hdweap_medical_base)
                        (Default|AltFire _asbp_hdweap_medical_base)
                        (Default|OnPCFirePressed _asbp_hdplayer_character_base)))
                    (:CastFailed
                      ;[1 0 0] Probably Don't need this for base controller
                      (Class|DFBaseCharacter|AimToggle _asbp_hdplayer_character_base)))))))))))
  (:Released
    (bind _asbp_hdplayer_character_base_2 (Utilities|Casting|CastToBP_HDPlayerCharacterBase (Pawn|GetControlledPawn)))
    (bind _asbp_hdweap_medical_base_2 (Utilities|Casting|CastToBP_HDWeap_MedicalBase (Class|DFBaseCharacter|GetEquippedItem _asbp_hdplayer_character_base_2)))
    (if (Variables|/HDCore/Core/Items/BP_HDWeap_MedicalBase.BP_HDWeap_MedicalBase_C|GetAltFIreEnabled _asbp_hdweap_medical_base_2)
      (Default|OnPCFireReleased _asbp_hdplayer_character_base))))

(event Input|ActionEvents|InputActionPauseMenu
  (params (Key :type Key%20Structure :default "None"))
  ;[1 1 1] Removes Radial Menu if Pause Menu is pressed
  (:Pressed
    (CallFunction|EndInteraction)))

(fn ConstructionScript
  (|CallParentFunction))

(fn DeployMenuToggle
  (params (bShowMenu :type Boolean) (bForce :type Boolean))
  (CallFunction|EndInteraction)
  (|CallParentFunction bShowMenu bForce))

(fn SetResupplyCooldownTimestap
  (Variables|Resupply|SetResupplyCooldownTimeStamp (GameState|GetServerWorldTimeSeconds (CallFunction|GetHDGameState))))