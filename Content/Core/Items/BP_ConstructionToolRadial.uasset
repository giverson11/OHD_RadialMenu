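; Construction tool item that opens a radial menu when the player interacts with it.
; Interact calls DisplayRadialMenu on the InteractibleComponent, and unequipping runs the parent logic, then hides the menu where cosmetic events can execute.
; CanShowWidget always returns false.
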(event EventBeginPlay)

(event Collision|EventActorBeginOverlap
  (params (OtherActor :type Actor%20Object%20Reference)))

(event EventTick
  (params (DeltaSeconds :type Float%20%28single-precision%29))
  (|CallParentFunction DeltaSeconds) ; This node is disabled and will not be called.\nDrag off pins to build functionality.
)

(event EventInteract
  (params (InstigatingController :type BP%20HD%20Player%20Controller%20Base%20Object%20Reference))
  (Default|DisplayRadialMenu (Variables|Default|GetInteractibleComponent)))

(event EventOnUnEquip
  (params (bPlayAnimAndWait :type Boolean) (bLeavingPawnInventory :type Boolean))
  (|CallParentFunction bPlayAnimAndWait bLeavingPawnInventory)
  (Networking|CanExecuteCosmeticEvents
    (:True
      (Default|HideRadialMenu (Variables|Default|GetInteractibleComponent)))))

(fn ConstructionScript
  (|CallParentFunction))

(fn CanShowWidget
  (return false))